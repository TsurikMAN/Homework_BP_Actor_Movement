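; BP_Ball is a ball actor that travels on its own and bounces off whatever it hits.
; Each Tick it moves its Sphere component by direction, speed and delta time with a swept world offset.
; On a blocking hit it reflects the direction around the surface normal and cuts speed by a fraction, as long as speed is at or above a Lowest threshold.
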(event EventBeginPlay)

(event Collision|EventActorBeginOverlap
  (params (OtherActor :type Actor%20Object%20Reference)))

(event EventTick
  (params (DeltaSeconds :type Float%20%28single-precision%29))
  (bind _sweephitresult (Transformation|AddWorldOffset (Variables|Default|GetSphere) (* (* (Variables|Default|GetDirections) (Variables|Default|GetSpeed)) DeltaSeconds) true false))
  (if (.bBlockingHit (Collision|BreakHitResult _sweephitresult))
    (if (>= (Variables|Default|GetSpeed) (Variables|Default|GetLowest))
      (Variables|Default|SetSpeed (* (Variables|Default|GetSpeed) 0.9)))
    (Variables|Default|SetDirections (Math|Vector|GetReflectionVector (Variables|Default|GetDirections) (.Normal (Collision|BreakHitResult _sweephitresult))))))

(fn ConstructionScript)